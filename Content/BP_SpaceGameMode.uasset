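; BP_SpaceGameMode is the game mode for a space game, managing the HUD and the game-over screen.
; On BeginPlay it adds WBP_HUD to the viewport, hides the mouse cursor and sets game-only input.
; OnGameOver creates and shows a game-over widget, shows the cursor, switches input to UI-only focused on that widget, and pauses the game.
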(event `self.OnGameOver`
  (bind _returnvalue (`GameplayStatics.GetPlayerController` 0))
  (bind _returnvalue_2 (`|CreateWidget` "/Game/WBP_GameOver.WBP_GameOver_C" _returnvalue))
  (`UserWidget.AddToViewport` _returnvalue_2 0)
  (set `PlayerController.bShowMouseCursor` true _returnvalue)
  (`WidgetBlueprintLibrary.SetInputMode_UIOnlyEx` _returnvalue _returnvalue_2)
  (`GameplayStatics.SetGamePaused` true))

(event `self.ReceiveBeginPlay`
  (bind _returnvalue (`GameplayStatics.GetPlayerController` 0))
  (bind _returnvalue_2 (`|CreateWidget` "/Game/WBP_HUD.WBP_HUD_C" (`GameplayStatics.GetPlayerController` 0)))
  (`UserWidget.AddToViewport` _returnvalue_2 0)
  (set `PlayerController.bShowMouseCursor` false _returnvalue)
  (`WidgetBlueprintLibrary.SetInputMode_GameOnly` _returnvalue))

(fn `UserConstructionScript`)